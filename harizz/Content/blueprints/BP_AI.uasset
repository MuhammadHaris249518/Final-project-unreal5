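; BP_AI is an enemy that chases the first player on sight and knocks characters back with a melee attack.
; PawnSensing triggers AI MoveTo; on arrival it plays the attack montage.
; Montage notifies, completion and interruption each fire a short forward sphere trace, launching any hit Character forward and upward by knockback variables.
; CanATTACK is toggled around the montage but never gates attacks.
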(event OnSeePawn(PawnSensing)
  (params (Pawn :type Pawn%20Object%20Reference))
  (CallFunction|ChasePlayers))

(event Custom|chase_players
  (bind _returnvalue (Transformation|GetActorLocation))
  (AI|AIMoveTo self "0, 0, 0" (Game|GetPlayerCharacter 0) 1.2e+02 false
    (:OnSuccess
      (if true
        (Animation|Montage|PlayMontage (Variables|Character|GetMesh) "/Game/Characters/Villager/Animations/attack/attack_Montage.attack_Montage"
          (:then
            (Variables|Default|SetcanATTACK? false))
          (:OnCompleted
            (Variables|Default|SetcanATTACK? true :!label _label)
            (bind _outhit (Collision|SphereTraceByChannel _returnvalue (+ _returnvalue (* (Math|Vector|GetForwardVector (Transformation|GetActorRotation)) 1.8e+02)) 25.0 "TraceTypeQuery3" false 0 "None" true "(R=1.000000,G=0.000000,B=0.000000,A=1.000000)" "(R=0.000000,G=1.000000,B=0.000000,A=1.000000)" 0.5 :!label _label_2))
            (if true
              (bind _ascharacter (Utilities|Casting|CastToCharacter (.HitActor (Collision|BreakHitResult _outhit))))
              (Character|LaunchCharacter _ascharacter (+ (* (Math|Vector|GetForwardVector (Transformation|GetActorRotation)) (Variables|Default|GetFrontalknockback)) (Math|Vector|MakeVector 0.0 0.0 (Variables|Default|GetUpwardsknockback))) false false)))
          (:OnInterrupted
            (goto _label))
          (:OnNotifyBegin
            (goto _label_2)))))))

(event EventBeginPlay)

(fn ConstructionScript)